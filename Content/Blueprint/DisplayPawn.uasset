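; DisplayPawn is a pawn with a mouse-rotated spring arm, apparently for viewing a displayed model.
; MouseX and MouseY feed yaw and pitch straight into the arm's relative rotation, with no clamping.
; BeginPlay calls CreateMesh to add a static mesh component at runtime.
; A separate Func, not called in this graph, spawns a BP_Drone with tick disabled and snaps it on as an attachment.
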(event EventBeginPlay
  (CallFunction|CreateMesh))

(event Collision|EventActorBeginOverlap
  (params (OtherActor :type Actor%20Object%20Reference)))

(event EventTick
  (params (DeltaSeconds :type Float%20%28single-precision%29)))

(event Input|AxisEvents|InputAxisMouseX
  (params (AxisValue :type Float%20%28single-precision%29))
  (Transformation|AddRelativeRotation (Variables|Default|GetSpringArm) (Math|Rotator|MakeRotator 0.0 0.0 AxisValue) false false))

(event Input|AxisEvents|InputAxisMouseY
  (params (AxisValue :type Float%20%28single-precision%29))
  (Transformation|AddRelativeRotation (Variables|Default|GetSpringArm) (Math|Rotator|MakeRotator 0.0 AxisValue 0.0) false false))

(fn ConstructionScript)

(fn Func
  (bind _returnvalue (Game|SpawnActorfromClass "/Game/Blueprint/BP_Drone.BP_Drone_C" (Math|Transform|MakeTransform "0, 0, 0") "AlwaysSpawn" 0 0))
  (Actor|Tick|SetActorTickEnabled _returnvalue)
  (Transformation|AttachComponentToComponent _returnvalue 0 "None" "SnapToTarget" "SnapToTarget" "SnapToTarget" false)
  (Transformation|SetActorRelativeTransform _returnvalue (Math|Transform|MakeTransform "0, 0, 0") false false))

(fn CreateMesh
  (AddComponent|AddStaticMeshComponent false))